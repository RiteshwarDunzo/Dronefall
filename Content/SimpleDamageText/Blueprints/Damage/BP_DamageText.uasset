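; BP_DamageText is a short-lived actor that shows a floating damage number in the game.
; On BeginPlay it passes the truncated Damage value to its UI_DamageText widget component.
; A timeline then lerps the actor from its spawn location to a fixed raised, sideways offset, and the actor destroys itself when the timeline finishes.
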(event `self.ReceiveBeginPlay`
  ;[1 0.1146 0.1146] DAMAGGE INDICATOR
  (bind _asui_damage_text (cast `/Game/SimpleDamageText/Blueprints/UI/UI_DamageText` (`WidgetComponent.GetWidget` (`self.UI_DamageText`))))
  (set `/Game/SimpleDamageText/Blueprints/UI/UI_DamageText.damage` (`KismetMathLibrary.FTrunc` (`self.Damage`)) _asui_damage_text)
  (bind _output_get (set `self.startLocation` (`self.K2_GetActorLocation`)))
  (set `self.endLocation` (+ _output_get (-25.0 -25.0 50.0)))
  (bind (_direction _move_track) (`Timeline|TimelineDamageIndicator`)
    (:`Update`
      (`self.K2_SetActorLocation` (`KismetMathLibrary.VLerp` (`self.startLocation`) (`self.endLocation`) _move_track)))
    (:`Finished`
      (`self.K2_DestroyActor`))))

(fn `UserConstructionScript`)