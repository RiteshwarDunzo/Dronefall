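; Player drone pawn that flies, looks and fires blaster beams, with an overlay HUD.
; Enhanced Input drives FloatingPawnMovement along control-rotation axes and turns the controller, whose rotation the drone mesh copies every tick.
; Firing alternates left and right rifle sockets, using a debug-drawn camera trace to aim each spawned beam at the crosshair point, with sound and Niagara burst.
; GetHurt subtracts health and quits the game at zero.
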(event `self.ReceiveTick`
  (params (DeltaSeconds :type "Float (single-precision)"))
  ;[1 0.09573 0.09138 0.5] Drone Look
  (`self.RotateMeshToController`))

(event `self.ReceiveBeginPlay`
  ; Pawn Input Mapping Context
  (`self.AddInputMappingContext`)
  (bind _returnvalue (`|CreateWidget` "/Game/Assets/UI/WBP_OverlayHUD.WBP_OverlayHUD_C"))
  (`UserWidget.AddToViewport` _returnvalue 0))

(event `EnhancedInput|/Game/Assets/Input/InputActions/IA_Fire`
  (params (ActionValue :type Boolean) (ElapsedSeconds :type "Float (double-precision)") (TriggeredSeconds :type "Float (double-precision)") (InputAction :type "InputAction Object Reference" :default "/Game/Assets/Input/InputActions/IA_Fire.IA_Fire"))
  ;[0 0.02357 0.15 0.5 25] PAWN INPUT HANDLING
  ;; Pawn Firing
  (:`Triggered`
    (bind _isa (`/Engine/EditorBlueprintResources/StandardMacros.FlipFlop`)
      (:`A`
        _)
      (:`B`
        _))
    (`self.FireRifle` _isa)))

(event `EnhancedInput|/Game/Assets/Input/InputActions/IA_Look`
  (params (ActionValue :type "Vector2D Structure") (ElapsedSeconds :type "Float (double-precision)") (TriggeredSeconds :type "Float (double-precision)") (InputAction :type "InputAction Object Reference" :default "/Game/Assets/Input/InputActions/IA_Look.IA_Look"))
  ;[0 0.02357 0.15 0.5 25] PAWN INPUT HANDLING
  ;; Pawn Look
  (:`Triggered`
    (`self.HandlePawnLook` ActionValue)))

(event `EnhancedInput|/Game/Assets/Input/InputActions/IA_Move`
  (params (ActionValue :type "Vector Structure") (ElapsedSeconds :type "Float (double-precision)") (TriggeredSeconds :type "Float (double-precision)") (InputAction :type "InputAction Object Reference" :default "/Game/Assets/Input/InputActions/IA_Move.IA_Move"))
  ;[0 0.02357 0.15 0.5 25] PAWN INPUT HANDLING
  ;; Pawn Moving
  (:`Triggered`
    (`self.HandleFloatingPawnMovement`)))

(event `/Game/BlueprintInterfaces/BI_Damageable.Get Hurt`
  (params (Damage :type "Float (double-precision)"))
  (bind _output_get (set `self.Health` (- (`self.Health`) Damage)))
  (`KismetSystemLibrary.PrintString` (`KismetStringLibrary.Concat_StrStr` "Health : " (`KismetStringLibrary.Conv_DoubleToString` _output_get)))
  (if (<= (`self.Health`) 0.0)
    (`KismetSystemLibrary.QuitGame` null "Quit")))

(fn `AddInputMappingContext`
  (cast `PlayerController` (`self.GetController`))
  (`EnhancedInputSubsystemInterface.AddMappingContext` (subsystem `EnhancedInputLocalPlayerSubsystem`) "/Game/Assets/Input/IMC_Drone.IMC_Drone" 0 (struct)))

(fn `FireRifle`
  (params (IsLeftRifle :type Boolean :default false))
  (locals (TraceEnd :type "Vector Structure"))
  (set `local.TraceEnd` (`self.GetTraceEnd`))
  (bind _outhit (`KismetSystemLibrary.LineTraceSingle` :`Start` (`SceneComponent.K2_GetComponentLocation` (`self.Camera`)) :`End` (`local.TraceEnd`) :`TraceChannel` "TraceTypeQuery1" :`DrawDebugType` "ForDuration" :`TraceHitColor` (struct :`R` 0.012041 :`B` 1.0 :`A` 1.0) :`DrawTime` 60.0))
  (bind (_bblockinghit _binitialoverlap _time _distance _location _impactpoint) (`GameplayStatics.BreakHitResult` _outhit))
  (set `local.TraceEnd` (`KismetMathLibrary.SelectVector` _impactpoint (`local.TraceEnd`) _bblockinghit))
  (if (`local.IsLeftRifle`)
    (set `self.Socket Name` "Rifle_L")
    (else
      (set `self.Socket Name` "Rifle_R")))
  (`|SpawnActorFromClass` "/Game/Blueprints/BP_PlayerBlasterBeam_Child.BP_PlayerBlasterBeam_Child_C" (`self.GetSpawnTransform` (`local.TraceEnd`)) "Undefined" "MultiplyWithRoot" null null null)
  (`self.SpawnFireEffects`))

(fn `GetForwardInputVector`
  (returns (Y :type "Float (double-precision)") (ReturnValue :type "Vector Structure"))
  (return (.y (`|GetInputActionValue`)) (`KismetMathLibrary.GetForwardVector` (`self.GetControlRotation`))))

(fn `GetRightInputVector`
  (returns (X :type "Float (double-precision)") (ReturnValue :type "Vector Structure"))
  (return (.x (`|GetInputActionValue`)) (`KismetMathLibrary.GetRightVector` (`self.GetControlRotation`))))

(fn `GetSpawnTransform`
  (params (TraceEnd :type "Vector Structure (by ref)"))
  (returns (ReturnValue :type "Transform Structure"))
  (bind _returnvalue_location (`KismetMathLibrary.BreakTransform` (`SceneComponent.GetSocketTransform` (`self.DroneMesh`) (`self.Socket Name`) "RTS_World")))
  (return (`KismetMathLibrary.MakeTransform` _returnvalue_location (`KismetMathLibrary.FindLookAtRotation` _returnvalue_location (`local.TraceEnd`)))))

(fn `GetTraceEnd`
  (returns (ReturnValue :type "Vector Structure"))
  (bind _camera (`self.Camera`))
  (return (+ (`SceneComponent.K2_GetComponentLocation` _camera) (* (`SceneComponent.GetForwardVector` _camera) (`self.TraceDistance`)))))

(fn `GetUpInputVector`
  (returns (Z :type "Float (double-precision)") (ReturnValue :type "Vector Structure"))
  (return (.z (`|GetInputActionValue`)) (`KismetMathLibrary.GetUpVector` (`self.GetControlRotation`))))

(fn `HandleFloatingPawnMovement`
  (bind (_x _returnvalue) (`self.GetRightInputVector`))
  (bind (_y _returnvalue_2) (`self.GetForwardInputVector`))
  (bind (_z _returnvalue_3) (`self.GetUpInputVector`))
  (`PawnMovementComponent.AddInputVector` (`self.FloatingPawnMovement`) (* _x _returnvalue) false)
  (`PawnMovementComponent.AddInputVector` (`self.FloatingPawnMovement`) (* _y _returnvalue_2) false)
  (`PawnMovementComponent.AddInputVector` (`self.FloatingPawnMovement`) (* _z _returnvalue_3) false))

(fn `HandlePawnLook`
  (params (`Action Value` :type "Vector2D Structure"))
  (bind (_x _y) (`KismetMathLibrary.BreakVector2D` `Action Value`))
  (`self.AddControllerYawInput` _x)
  (`self.AddControllerPitchInput` _y))

(fn `RotateMeshToController`
  (`SceneComponent.K2_SetWorldRotation` (`self.DroneMesh`) (`self.GetControlRotation`) false false))

(fn `SpawnFireEffects`
  (bind (_returnvalue_location _returnvalue_rotation _returnvalue_scale) (`KismetMathLibrary.BreakTransform` (`SceneComponent.GetSocketTransform` (`self.DroneMesh`) (`self.Socket Name`) "RTS_World")))
  (`GameplayStatics.PlaySoundAtLocation` "/Game/Assets/Sounds/Drone/Sfx_EnergyRifle.Sfx_EnergyRifle" (`SceneComponent.GetSocketLocation` (`self.DroneMesh`) (`self.Socket Name`)) (struct) 1.0 1.0 0.0 "/Game/Assets/Sounds/Drone/Att_EnergyRifle.Att_EnergyRifle" null null null)
  (`NiagaraFunctionLibrary.SpawnSystemAtLocation` "/Game/Assets/FX/NS_BeamBurst.NS_BeamBurst" _returnvalue_location _returnvalue_rotation _returnvalue_scale))

(fn `UserConstructionScript`)