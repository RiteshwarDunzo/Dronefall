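; BP_SmallSphere is a moving, spinning pickup sphere that scores a point through BP_DronefallGameMode when a Pawn overlaps it.
; Tick moves it along its forward vector while applying a random spin, so its heading changes as it rotates.
; After Lifetime, a WinkIn scale timeline plays, then triggers WinkOut.
; Pawn overlap also triggers WinkOut, a scale timeline guarded by IsWinking that destroys the actor when finished.
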(event `self.ReceiveBeginPlay`
  (`self.InitializeDeltaRotation`)
  ; WinkIn Timeline
  (`KismetSystemLibrary.K2_SetTimerDelegate` (delegate `WinkIn`) (`self.Lifetime`))
  ; Handles Overlap
  (add `PrimitiveComponent.OnComponentBeginOverlap` (`self.SphereVolume`) (delegate `OnSphereOverlap`)))

(event `OnSphereOverlap`
  (params (OverlappedComponent :type "PrimitiveComponent Object Reference") (OtherActor :type "Actor Object Reference") (OtherComp :type "PrimitiveComponent Object Reference") (OtherBodyIndex :type Integer) (bFromSweep :type Boolean) (SweepResult :type "HitResult Structure (by ref)"))
  ; Handles Overlap
  (`KismetSystemLibrary.PrintString` (`KismetSystemLibrary.GetDisplayName` OtherActor))
  (if (`GameplayStatics.ObjectIsA` OtherActor "/Script/Engine.Pawn")
    (`self.WinkOut`)
    (bind _asbp_dronefall_game_mode (cast `/Game/Blueprints/BP_DronefallGameMode` (`GameplayStatics.GetGameMode`)))
    (`/Game/Blueprints/BP_DronefallGameMode.Incement Score` _asbp_dronefall_game_mode)))

(event `WinkIn`
  ; WinkIn Timeline
  (bind (_direction _scale) (`Timeline|WinkIn Timeline`)
    (:`Update`
      (`SceneComponent.SetWorldScale3D` (`self.SphereMesh`) _scale))
    (:`Finished`
      (`self.WinkOut`))))

(event `WinkOut`
  ; WinkOut Timeline
  (if (not (`self.IsWinking`))
    (set `self.IsWinking` true)
    (bind (_direction _scale) (`Timeline|WinkOut Timeline`)
      (:`Update`
        (`SceneComponent.SetWorldScale3D` (`self.SphereMesh`) (`KismetMathLibrary.Conv_DoubleToVector` _scale)))
      (:`Finished`
        (`self.K2_DestroyActor`)))))

(event `self.ReceiveTick`
  (params (DeltaSeconds :type "Float (single-precision)"))
  ;[1 0.09573 0.09138 0.5] Update Rotation and Location
  (`self.UpdateLocation` DeltaSeconds)
  (`self.UpdateRotation` DeltaSeconds))

(fn `InitializeDeltaRotation`
  (set `self.Delta Rotation` (* (`KismetMathLibrary.RandomRotator` false) (`self.RotationScaleFactor`))))

(fn `Scale`
  (params (Scale :type "Float (double-precision)"))
  (`SceneComponent.SetWorldScale3D` (`self.SphereMesh`) (`KismetMathLibrary.MakeVector` Scale Scale Scale)))

(fn `UpdateLocation`
  (params (`Delta Seconds` :type "Float (double-precision)"))
  (`self.K2_AddActorWorldOffset` (* (`self.GetActorForwardVector`) (* `Delta Seconds` (`self.Speed`)))))

(fn `UpdateRotation`
  (params (`Delta Seconds` :type "Float (single-precision)"))
  (`self.K2_AddActorWorldRotation` (* (`self.Delta Rotation`) `Delta Seconds`)))

(fn `UserConstructionScript`)