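; Spawner actor that periodically creates BP_SmallSphere actors at random points within a radius around itself.
; On BeginPlay, a looping timer fires at SpawnTime intervals and calls SpawnSmallSphere.
; Each spawn location is a random direction from a random rotator, scaled by a random distance up to SphereRadius and offset from the spawner's position.
; Each new sphere also receives a random rotation.
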(event `self.ReceiveBeginPlay`
  ; Start Sphere Spawn Timer
  (`KismetSystemLibrary.K2_SetTimerDelegate` (delegate `SpawnSphere`) (`self.SpawnTime`) true))

(event `SpawnSphere`
  ; Start Sphere Spawn Timer
  (`self.Spawn SmallSphere`))

(fn `Get Random Point In Sphere Radius`
  (returns (RandomPoint :type "Vector Structure"))
  (locals (NewLocalVar :type "Vector Structure"))
  (return (+ (`self.K2_GetActorLocation`) (* (`KismetMathLibrary.GetForwardVector` (`KismetMathLibrary.RandomRotator` false)) (`KismetMathLibrary.RandomFloatInRange` 0.0 (`self.SphereRadius`))))))

(fn `Spawn SmallSphere`
  (`|SpawnActorFromClass` "/Game/Blueprints/BP_SmallSphere.BP_SmallSphere_C" (`KismetMathLibrary.MakeTransform` (`self.Get Random Point In Sphere Radius`) (`KismetMathLibrary.RandomRotator` false)) "Undefined" "MultiplyWithRoot" null null))

(fn `UserConstructionScript`)